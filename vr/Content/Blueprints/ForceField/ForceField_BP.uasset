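; Force field Blueprint that shows a material-driven impact effect wherever its collision sphere is hit.
; Each hit creates a dynamic material instance on the Field component, passes it the impact point and spawns a debris emitter oriented along the impact normal.
; A timeline restarts on every hit, animating the material's "rad" parameter scaled by Radius and feeding Radius itself into "irad".
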(event OnComponentHit(SphereCollistion)
  (params (HitComponent :type Primitive%20Component%20Object%20Reference) (OtherActor :type Actor%20Object%20Reference) (OtherComp :type Primitive%20Component%20Object%20Reference) (NormalImpulse :type Vector :default "0, 0, 0") (Hit :type Hit%20Result%20Structure%20%28by%20ref%29))
  (bind _radius (Variables|Default|GetRadius))
  (bind _returnvalue (Rendering|Material|CreateDynamicMaterialInstance (Variables|Default|GetField) 0 0 :!class /Script/Engine.PrimitiveComponent))
  (Rendering|Material|SetVectorParameterValue _returnvalue "pos" (Math|Conversions|ToLinearColor(Vector) (.impactpoint Hit)) :!class /Script/Engine.MaterialInstanceDynamic)
  (Effects|SpawnEmitteratLocation "/Game/Blueprints/ForceField/Debri.Debri" (.impactpoint Hit) (Math|Rotator|MakeRotfromX (.impactnormal Hit)))
  (bind _newtrack_0 (Timeline|Animate PlayFromStart)
    (:Update
      (Rendering|Material|SetScalarParameterValue _returnvalue "rad" (* _newtrack_0 (* 1e+01 _radius)) :!class /Script/Engine.MaterialInstanceDynamic)
      (Rendering|Material|SetScalarParameterValue _returnvalue "irad" _radius :!class /Script/Engine.MaterialInstanceDynamic))))

(fn ConstructionScript)