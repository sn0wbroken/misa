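; TestGun is a gun Blueprint whose Shoot event spawns an enlarged TestBullet at the gun mesh's Muzzle socket.
; When unlocked, the shot follows the muzzle's rotation; otherwise it aims from the muzzle at the locked target's location.
; Both rotations pass through Ballistic with a narrow range for spread, though the random-rotator combine in that graph is marked unused.
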(event Custom|Shoot
  (params (IsUnLocked :type Boolean) (LockedTarget :type Actor%20Object%20Reference))
  (bind _gunmesh (Variables|Default|GetGunMesh))
  (bind _returnvalue (Transformation|GetSocketTransform _gunmesh "Muzzle" "RTS_World"))
  (if IsUnLocked
    (Game|SpawnActorfromClass "/Game/Blueprints/TestBullet.TestBullet_C" (Math|Transform|MakeTransform (.location _returnvalue) (Utilities|Ballistic (.rotation _returnvalue) -1.5 1.5) "20.000000,20.000000,20.000000") "Undefined" 0 0)
    (else
      (Game|SpawnActorfromClass "/Game/Blueprints/TestBullet.TestBullet_C" (Math|Transform|MakeTransform (.location _returnvalue) (Utilities|Ballistic (Math|Rotator|FindLookatRotation (.location _returnvalue) (Transformation|GetActorLocation LockedTarget)) -1.5 1.5) "20.000000,20.000000,20.000000") "Undefined" 0 0))))

(fn ConstructionScript)