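; MISA is a VR actor with arms that follow the player's motion controllers.
; Call snaps it onto the player pawn, caches controller references from MISAStateBase, and opens a Tick gate.
; Tick interpolates arm location and rotation variables toward scaled, offset controller transforms, and copies grip states into the A_BP_Arms animation instance.
; Rotation interpolation has its DeltaTime and InterpSpeed inputs swapped.
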(event Custom|Call
  (bind _returnvalue (Game|Player|GetPlayerPawn 0))
  (Transformation|SetActorLocationAndRotation (- (Transformation|GetActorLocation _returnvalue) "100.000000,0.000000,250.000000") (Transformation|GetActorRotation _returnvalue))
  (Transformation|AttachActorToActor _returnvalue "None" "SnapToTarget" "SnapToTarget" "KeepWorld" true)
  (bind _asmisastate_base (Utilities|Casting|CastToMISAStateBase (Game|GetGameState))
    (:then
      (Variables|Default|SetControllerL (Variables|/Game/Blueprints/MISAStateBase.MISAStateBase_C|GetController_L _asmisastate_base))
      (Variables|Default|SetControllerR (Variables|/Game/Blueprints/MISAStateBase.MISAStateBase_C|GetController_R _asmisastate_base))
      (CallFunction|Called))
    (:CastFailed
      (Development|PrintString "Cast Controller Transform Failled"))))

(event Custom|Called
  (bind _returnvalue (Utilities|Time|GetWorldDeltaSeconds))
  (bind _returnvalue_2 (Utilities|Time|GetWorldDeltaSeconds))
  (Utilities|FlowControl|Gate true) ; enters at Open
)

(event EventTick
  (params (DeltaSeconds :type Float%20%28single-precision%29))
  (bind _returnvalue (Utilities|Time|GetWorldDeltaSeconds))
  (bind _returnvalue_2 (Utilities|Time|GetWorldDeltaSeconds))
  (Utilities|FlowControl|Gate true
    (:Exit
      (Utilities|FlowControl|Sequence
        (:then_0
          ;[1 1 1] ARM sync & Interp left
          (Variables|Default|SetL_ARMLocation (Math|Interpolation|VInterpTo (Variables|Default|GetL_ARMLocation) (+ (+ "0, 0, 0" "1000.000000,-150.000000,100.000000") (* (.location (Transformation|GetRelativeTransform (Variables|Default|GetControllerL))) "10.000000,10.000000,10.000000")) _returnvalue_2 2.5))
          (Variables|Default|SetL_ARMRotation (Math|Interpolation|RInterpTo (Variables|Default|GetL_ARMRotation) (Transformation|GetWorldRotation (Variables|Default|GetControllerL)) 3.0 _returnvalue_2)))
        (:then_1
          ;[1 1 1] ARM sync & Interp right
          (Variables|Default|SetR_ARMLocation (Math|Interpolation|VInterpTo (Variables|Default|GetR_ARMLocation) (+ (+ "0, 0, 0" "1000.000000,150.000000,100.000000") (* (.location (Transformation|GetRelativeTransform (Variables|Default|GetControllerR))) "10.000000,10.000000,10.000000")) _returnvalue 2.5))
          (Variables|Default|SetR_ARMRotation (Math|Interpolation|RInterpTo (Variables|Default|GetR_ARMRotation) (Transformation|GetWorldRotation (Variables|Default|GetControllerR)) 3.0 _returnvalue)))
        (:then_2
          (bind _asmotion_controller_pawn (Utilities|Casting|CastToMotionControllerPawn (Game|Player|GetPlayerPawn 0)))
          (bind _asa_bp_arms (Utilities|Casting|CastToA_BP_Arms (Components|SkeletalMesh|GetAnimInstance (Variables|Default|GetSkeletalMesh))))
          (Variables|/Game/Input/FPMesh/Animation/A_BP_Arms.A_BP_Arms_C|SetGripState_L _asa_bp_arms (Utilities|Enum|Equal(Enum) (Variables|/Game/VirtualRealityBP/Blueprints/BP_MotionController.BP_MotionController_C|GetGripState (Variables|/Game/VirtualRealityBP/Blueprints/MotionControllerPawn.MotionControllerPawn_C|GetLeftController _asmotion_controller_pawn)) "NewEnumerator2"))
          (Variables|/Game/Input/FPMesh/Animation/A_BP_Arms.A_BP_Arms_C|SetGripState_R _asa_bp_arms (Utilities|Enum|Equal(Enum) (Variables|/Game/VirtualRealityBP/Blueprints/BP_MotionController.BP_MotionController_C|GetGripState (Variables|/Game/VirtualRealityBP/Blueprints/MotionControllerPawn.MotionControllerPawn_C|GetRightController _asmotion_controller_pawn)) "NewEnumerator2")))))))

(fn ConstructionScript)