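; TestTarget is a lockable test target actor that explodes and destroys itself when hit.
; Hit spawns a scaled-up explosion at the hit location, clears the player IKpawn_BP's left and right enemy element references, then destroys the actor.
; TargetLockON and TargetLockOFF toggle an IsLockOn flag that drives custom depth rendering on the mesh as a lock-on visual.
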(event EventTargetLockON
  ;[1 1 1] TargetVisual Toggle
  (if (not (Variables|Default|GetIsLockOn))
    (bind _output_get (Variables|Default|SetIsLockOn true))
    (Rendering|SetRenderCustomDepth (Variables|Default|GetMesh) _output_get)))

(event EventTargetLockOFF
  ;[1 1 1] TargetVisual Toggle
  (bind _output_get (Variables|Default|SetIsLockOn false))
  (Rendering|SetRenderCustomDepth (Variables|Default|GetMesh) _output_get))

(event Collision|EventHit
  (params (MyComp :type Primitive%20Component%20Object%20Reference) (Other :type Actor%20Object%20Reference) (OtherComp :type Primitive%20Component%20Object%20Reference) (bSelfMoved :type Boolean) (HitLocation :type Vector :default "0, 0, 0") (HitNormal :type Vector :default "0, 0, 0") (NormalImpulse :type Vector :default "0, 0, 0") (Hit :type Hit%20Result%20Structure%20%28by%20ref%29))
  (bind _returnvalue (Effects|SpawnEmitteratLocation "/Game/StarterContent/Particles/P_Explosion.P_Explosion" HitLocation))
  (Transformation|SetWorldScale3D _returnvalue "3.000000,3.000000,3.000000")
  (bind _asikpawn_bp (Utilities|Casting|CastToIKpawn_BP (Game|GetPlayerCharacter 0)))
  (Variables|/Game/Blueprints/IKpawn_BP.IKpawn_BP_C|SetEnemyElement_L _asikpawn_bp 0)
  (Variables|/Game/Blueprints/IKpawn_BP.IKpawn_BP_C|SetEnemyElement_R _asikpawn_bp 0)
  (Actor|DestroyActor))

(fn ConstructionScript)