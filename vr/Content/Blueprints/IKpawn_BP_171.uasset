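; VR pawn with an IK-animated arm mesh that the player can grip with and summon or dismiss through a dissolve effect.
; Left and right grab inputs set grip booleans on FP_MeshIK_ABP, and a reset input recenters the headset.
; The summon input alternates two timelines driving dissolve on dynamic materials, toggling visibility and collision, with a gate blocking presses mid-transition.
; BeginPlay sets floor tracking origin and disables arm collision.
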(event Custom|Initialize%20Arm
  ;[1 1 1] Appear
  (Collision|SetCollisionEnabled (Variables|Default|GetArmMesh) "NoCollision"))

(event EventBeginPlay
  (Class|HeadMountedDisplayFunctionLibrary|SetTrackingOrigin "Floor")
  (CallFunction|InitializeArm))

(event Input|ActionEvents|InputActionResetVR
  (params (Key :type Key%20Structure))
  ;[1 1 1] Reset Orientation and Position
  (:Pressed
    (Class|HeadMountedDisplayFunctionLibrary|ResetOrientationandPosition 0.0 "OrientationAndPosition")))

(event Input|ActionEvents|InputActionGrabLeft
  (params (Key :type Key%20Structure))
  (bind _armmesh (Variables|Default|GetArmMesh))
  (bind _returnvalue (Components|SkeletalMesh|GetAnimInstance _armmesh))
  ;[0 0 0] Handle Controller Input
  (:Pressed
    (bind _asfp_mesh_ik_abp (Utilities|Casting|CastToFP_MeshIK_ABP _returnvalue))
    (Variables|/Game/Blueprints/FP_MeshIK_ABP.FP_MeshIK_ABP_C|SetGripState_L _asfp_mesh_ik_abp true))
  (:Released
    (bind _asfp_mesh_ik_abp_2 (Utilities|Casting|CastToFP_MeshIK_ABP _returnvalue))
    (Variables|/Game/Blueprints/FP_MeshIK_ABP.FP_MeshIK_ABP_C|SetGripState_L _asfp_mesh_ik_abp_2 false)))

(event Input|ActionEvents|InputActionGrabRight
  (params (Key :type Key%20Structure))
  (bind _armmesh (Variables|Default|GetArmMesh))
  (bind _returnvalue (Components|SkeletalMesh|GetAnimInstance _armmesh))
  ;[0 0 0] Handle Controller Input
  (:Pressed
    (bind _asfp_mesh_ik_abp (Utilities|Casting|CastToFP_MeshIK_ABP _returnvalue))
    (Variables|/Game/Blueprints/FP_MeshIK_ABP.FP_MeshIK_ABP_C|SetGripState_R _asfp_mesh_ik_abp true))
  (:Released
    (bind _asfp_mesh_ik_abp_2 (Utilities|Casting|CastToFP_MeshIK_ABP _returnvalue))
    (Variables|/Game/Blueprints/FP_MeshIK_ABP.FP_MeshIK_ABP_C|SetGripState_R _asfp_mesh_ik_abp_2 false)))

(event Input|ActionEvents|InputActionARMSummon
  (params (Key :type Key%20Structure))
  (bind _armmesh (Variables|Default|GetArmMesh))
  (bind _armmesh_2 (Variables|Default|GetArmMesh))
  (bind _armmesh_3 (Variables|Default|GetArmMesh))
  ;[1 1 1] Appear
  (:Pressed
    (Utilities|FlowControl|Gate false :!label _label
      (:Exit
        (Utilities|FlowControl|Sequence
          (:then_0
            (goto _label Close))
          (:then_1
            (bind _returnvalue (Rendering|Material|CreateDynamicMaterialInstance _armmesh 0 "/Game/Material/M_Dissolve_ARM.M_Dissolve_ARM" :!class /Script/Engine.PrimitiveComponent))
            (bind _returnvalue_2 (Rendering|Material|CreateDynamicMaterialInstance _armmesh 1 "/Game/Material/M_Dissolve_ARM.M_Dissolve_ARM" :!class /Script/Engine.PrimitiveComponent))
            (Utilities|FlowControl|FlipFlop
              (:A
                (Rendering|SetVisibility _armmesh_3 true false)
                (Utilities|FlowControl|Sequence
                  (:then_0
                    (bind _arise (Timeline|Timeline_0 SetNewTime)
                      (:Update
                        (Rendering|Material|SetScalarParameterValue _returnvalue "Dissolve Amount" _arise :!class /Script/Engine.MaterialInstanceDynamic))
                      (:Finished
                        (Collision|SetCollisionEnabled _armmesh_2 "QueryAndPhysics")
                        (goto _label Open))))
                  (:then_1
                    (Timeline|Timeline_0 Play))))
              (:B
                (Collision|SetCollisionEnabled _armmesh_3 "NoCollision")
                (Utilities|FlowControl|Sequence
                  (:then_0
                    (bind _dissolve (Timeline|Timeline_1 SetNewTime)
                      (:Update
                        (Rendering|Material|SetScalarParameterValue _returnvalue_2 "Dissolve Amount" _dissolve :!class /Script/Engine.MaterialInstanceDynamic))
                      (:Finished
                        (Rendering|SetVisibility _armmesh_2 false false)
                        (goto _label Open))))
                  (:then_1
                    (Timeline|Timeline_1 Play)))))))))))

(fn ConstructionScript)