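; ExploadeSpawn is a spawner actor that keeps creating ExplodeEnemy characters during play.
; On BeginPlay, after a validity check, a looping Delay spawns one every few seconds with no count limit.
; Each appears at a random point on the line between referenced actor A and the spawner, with random rotation and enlarged scale, then has its CharacterMovement activated.
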(event EventBeginPlay
  (if (Variables|Default|GetbValid)
    (Utilities|FlowControl|Delay 3.0 :!label _label)
    (bind _returnvalue (Game|SpawnActorfromClass "/Game/Blueprints/ExplodeEnemy.ExplodeEnemy_C" (Math|Transform|MakeTransform (Math|Vector|Lerp(Vector) (Transformation|GetActorLocation (Variables|Default|GetA)) (Transformation|GetActorLocation) (Math|Random|RandomFloat)) (Math|Random|RandomRotator false) "10.000000,10.000000,10.000000") "Undefined" 0 0))
    (Components|Activation|Activate (Variables|/Script/Engine.Character|GetCharacterMovement _returnvalue) false)
    (goto _label)))

(fn ConstructionScript)