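; Destructed shield actor that shatters a destructible mesh when it spawns and fades out the pieces.
; On BeginPlay it applies full radius damage to its Destructible, with radius and impulse scaled by the actor's scale.
; It creates dynamic material instances on both mesh slots, and a timeline played in reverse from the end drives their "vis" parameter.
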(event EventBeginPlay
  (bind _returnvalue (Transformation|GetActorScale3D))
  (bind _destructible (Variables|Default|GetDestructible))
  (bind _destructible_2 (Variables|Default|GetDestructible))
  (bind _returnvalue_2 (Math|Vector|VectorLength _returnvalue))
  (bind _returnvalue_3 (* _returnvalue_2 5e+02))
  (Class|DestructibleComponent|ApplyRadiusDamage _destructible_2 1e+01 (Transformation|GetWorldLocation _destructible_2) _returnvalue_3 _returnvalue_3 true)
  (bind _returnvalue_4 (Rendering|Material|CreateDynamicMaterialInstance _destructible 0 "/Game/Blueprints/ForceField/DestructedField_mat_Inst.DestructedField_mat_Inst" :!class /Script/Engine.PrimitiveComponent))
  (bind _returnvalue_5 (Rendering|Material|CreateDynamicMaterialInstance _destructible 1 "/Game/Blueprints/ForceField/DestructedField_mat_Inst.DestructedField_mat_Inst" :!class /Script/Engine.PrimitiveComponent))
  (bind _newtrack_0 (Timeline|Timeline_0 ReverseFromEnd)
    (:Update
      (Rendering|Material|SetScalarParameterValue _returnvalue_4 "vis" _newtrack_0 :!class /Script/Engine.MaterialInstanceDynamic)
      (Rendering|Material|SetScalarParameterValue _returnvalue_5 "vis" _newtrack_0 :!class /Script/Engine.MaterialInstanceDynamic))))

(fn ConstructionScript)