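; BaseTarget is a destructible, lockable target actor that tracks HP from incoming damage.
; At zero HP it spawns a scaled death emitter and sound, notifies the player character (IKpawn_BP) via DestroyedEnemyElementR, then destroys itself.
; Lock-on and lock-off events set IsLockOn and toggle the mesh's custom depth rendering as a visual marker, printing the state for debugging.
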(event EventTargetLockON
  ;[1 1 1] TargetVisual Toggle
  (if (not (Variables|Default|GetIsLockOn))
    (bind _output_get (Variables|Default|SetIsLockOn true))
    (Rendering|SetRenderCustomDepth (Variables|Character|GetMesh) _output_get)
    (Development|PrintString (Utilities|String|ToString(Boolean) (Variables|Default|GetIsLockOn)))))

(event Game|Damage|EventAnyDamage
  (params (Damage :type Float%20%28single-precision%29) (DamageType :type Damage%20Type%20Object%20Reference) (InstigatedBy :type Controller%20Object%20Reference) (DamageCauser :type Actor%20Object%20Reference))
  (bind _output_get (Variables|Default|SetHP (- (Variables|Default|GetHP) Damage)))
  (if (<= _output_get 0.0)
    (bind _returnvalue (Effects|SpawnEmitteratLocation (Variables|Default|GetDeadEmitter) (Transformation|GetActorLocation)))
    (Transformation|SetWorldScale3D _returnvalue (* (Transformation|GetActorScale3D) 5))
    (Audio|SpawnSoundatLocation (Variables|Default|GetDeadSound) (Transformation|GetActorLocation) "0, 0, 0" 1e+02 0.8)
    (bind _asikpawn_bp (Utilities|Casting|CastToIKpawn_BP (Game|GetPlayerCharacter 0))
      (:then
        (Default|DestroyedEnemyElementR _asikpawn_bp))
      (:CastFailed
        _))
    (Actor|DestroyActor)))

(event EventTargetLockOFF
  ;[1 1 1] TargetVisual Toggle
  (bind _output_get (Variables|Default|SetIsLockOn false))
  (Rendering|SetRenderCustomDepth (Variables|Character|GetMesh) _output_get)
  (Development|PrintString (Utilities|String|ToString(Boolean) (Variables|Default|GetIsLockOn))))

(fn ConstructionScript)