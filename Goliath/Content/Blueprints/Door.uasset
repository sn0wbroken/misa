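; A door actor that slides a Door component between its starting position and the position of a Destination component.
; BeginPlay caches both relative locations, then the DoorControll timeline's Rate track lerps the door between them.
; Open, Close and Stop events play, reverse and halt the timeline, so the door can change direction or pause mid-motion.
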(event Custom|Open
  (bind _rate (Timeline|DoorControll Play)
    (:Update
      (Transformation|SetRelativeLocation (Variables|Default|GetDoor) (Math|Vector|Lerp(Vector) (Variables|Default|GetInitial_position) (Variables|Default|GetDestination_Position) _rate) false false))))

(event Custom|Stop
  (bind _rate (Timeline|DoorControll Stop)
    (:Update
      (Transformation|SetRelativeLocation (Variables|Default|GetDoor) (Math|Vector|Lerp(Vector) (Variables|Default|GetInitial_position) (Variables|Default|GetDestination_Position) _rate) false false))))

(event Custom|Close
  (bind _rate (Timeline|DoorControll Reverse)
    (:Update
      (Transformation|SetRelativeLocation (Variables|Default|GetDoor) (Math|Vector|Lerp(Vector) (Variables|Default|GetInitial_position) (Variables|Default|GetDestination_Position) _rate) false false))))

(event EventBeginPlay
  (Variables|Default|SetInitial_position (.location (Transformation|GetRelativeTransform (Variables|Default|GetDoor))))
  (Variables|Default|SetDestination_Position (.location (Transformation|GetRelativeTransform (Variables|Default|GetDestination)))))

(fn ConstructionScript)