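; Energy-limited force shield actor that SetScale toggles open and closed with sound and a scale timeline.
; Projectile hits spawn debris and drive a material ripple from the impact point, sized by projectile radius.
; Looping timers drain energy while unfolded and recharge it through a gate while collapsed; damage also drains it.
; At zero energy it spawns DestructedShield_BP and collapses, pausing recharge for five seconds before partly refilling.
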(event Custom|SetScale
  (params (OriginalSize :type Vector))
  (bind _returnvalue (Transformation|GetActorLocation))
  (bind _energypoint (Variables|Default|GetEnergyPoint))
  (bind _shield_electro_loop_ver1_1 (Variables|Default|GetShield_electro-loop_ver1_1))
  (bind _returnvalue_2 (> _energypoint 0.0))
  ;[1 1 1] Set Scale
  (bind _isa (Utilities|FlowControl|FlipFlop)
    (:A
      (Variables|Default|SetUnfold _isa)
      (if _returnvalue_2
        (Audio|PlaySoundatLocation "/Game/Import/Shield/Shield_electro-Active.Shield_electro-Active" _returnvalue)
        (Components|Activation|SetActive _shield_electro_loop_ver1_1 true true)
        (bind _raidus (Timeline|EquipShield Play)
          (:Update
            (if (>= (Variables|Default|GetEnergyPoint) 0.0)
              (Transformation|SetActorScale3D (Math|Vector|Lerp(Vector) "0, 0, 0" OriginalSize _raidus)))))))
    (:B
      (Variables|Default|SetUnfold _isa)
      (if _returnvalue_2
        (Audio|PlaySoundatLocation "/Game/Import/Shield/Shield_electro-Deactive.Shield_electro-Deactive" _returnvalue)
        (Components|Activation|SetActive _shield_electro_loop_ver1_1 false true)
        (Timeline|EquipShield Reverse)))))

(event Custom|Charge
  ;[1 1 1] Charge
  (Utilities|Time|SetTimerbyEvent (delegate Custom|Charge) 0.1)
  (Utilities|FlowControl|Gate false
    (:Exit
      (if (and (== (Math|Vector|VectorLength (Transformation|GetActorScale3D)) 0.0) (< (Variables|Default|GetEnergyPoint) (Variables|Default|GetMaxEnergy)))
        (Variables|Default|SetEnergyPoint (+ (Variables|Default|GetEnergyPoint) (* (Variables|Default|GetMaxEnergy) 0.01)))))))

(event Custom|cost
  ;[1 1 1] Cost
  (Utilities|Time|SetTimerbyEvent (delegate Custom|cost) 0.1)
  (if (and (Variables|Default|GetUnfold) (> (Variables|Default|GetEnergyPoint) 0.0))
    (Math|Float|DecrementFloat (Variables|Default|GetEnergyPoint)
      (:%20%20
        ;[1 1 1] Energy Point
        (if (<= (Variables|Default|GetEnergyPoint) 0.0)
          (Game|SpawnActorfromClass "/Game/Blueprints/ForceField/DestructedShield_BP.DestructedShield_BP_C" (Transformation|GetActorTransform) "Undefined" 0 0)
          (Transformation|SetActorScale3D "0, 0, 0")
          (Utilities|FlowControl|Sequence
            (:then_0
              ;[1 1 1] Set Scale
              (Components|Activation|SetActive (Variables|Default|GetShield_electro-loop_ver1_1) false true)
              (bind _raidus (Timeline|EquipShield SetNewTime)
                (:Update
                  (if (>= (Variables|Default|GetEnergyPoint) 0.0)
                    (Transformation|SetActorScale3D (Math|Vector|Lerp(Vector) "0, 0, 0" (stale Custom|SetScale OriginalSize) _raidus))))))
            (:then_1
              ;[1 1 1] Charge
              (Utilities|FlowControl|Gate false) ; enters at Close
            )
            (:then_2
              ;[1 1 1] Be broken
              (Utilities|FlowControl|Delay 5.0)
              (Variables|Default|SetEnergyPoint (* (Variables|Default|GetMaxEnergy) 0.2))
              (Utilities|FlowControl|Gate false) ; enters at Open
            )))))))

(event Collision|EventHit
  (params (MyComp :type Primitive%20Component%20Object%20Reference) (Other :type Actor%20Object%20Reference) (OtherComp :type Primitive%20Component%20Object%20Reference) (bSelfMoved :type Boolean) (HitLocation :type Vector :default "0, 0, 0") (HitNormal :type Vector :default "0, 0, 0") (NormalImpulse :type Vector :default "0, 0, 0") (Hit :type Hit%20Result%20Structure%20%28by%20ref%29))
  ;[1 1 1] Hit shader
  (bind _asfirst_person_projectile (Utilities|Casting|CastToFirstPersonProjectile Other))
  (Variables|Default|SetRadius (Components|Sphere|GetScaledSphereRadius (Variables|/Game/FirstPersonBP/Blueprints/FirstPersonProjectile.FirstPersonProjectile_C|GetCollisionComponent _asfirst_person_projectile)))
  (Audio|PlaySoundatLocation "/Game/Import/Shield/Shield_electro-hit_.Shield_electro-hit_" (.impactpoint Hit))
  (bind _returnvalue (Rendering|Material|CreateDynamicMaterialInstance (Variables|Default|GetField) 0 0 :!class /Script/Engine.PrimitiveComponent))
  (Rendering|Material|SetVectorParameterValue _returnvalue "pos" (Math|Conversions|ToLinearColor(Vector) (.impactpoint Hit)) :!class /Script/Engine.MaterialInstanceDynamic)
  (Effects|SpawnEmitteratLocation "/Game/Blueprints/ForceField/Debri.Debri" (.impactpoint Hit) (Math|Rotator|MakeRotfromX (.impactnormal Hit)))
  (bind _newtrack_0 (Timeline|Point PlayFromStart)
    (:Update
      (Rendering|Material|SetScalarParameterValue _returnvalue "rad" (* _newtrack_0 (* 1e+01 (Variables|Default|GetRadius))) :!class /Script/Engine.MaterialInstanceDynamic)
      (Rendering|Material|SetScalarParameterValue _returnvalue "irad" (Variables|Default|GetRadius) :!class /Script/Engine.MaterialInstanceDynamic))))

(event Game|Damage|EventAnyDamage
  (params (Damage :type Float%20%28single-precision%29) (DamageType :type Damage%20Type%20Object%20Reference) (InstigatedBy :type Controller%20Object%20Reference) (DamageCauser :type Actor%20Object%20Reference))
  ;[1 1 1] Energy Point
  (Variables|Default|SetEnergyPoint (- (Variables|Default|GetEnergyPoint) Damage))
  (if (<= (Variables|Default|GetEnergyPoint) 0.0)
    (Game|SpawnActorfromClass "/Game/Blueprints/ForceField/DestructedShield_BP.DestructedShield_BP_C" (Transformation|GetActorTransform) "Undefined" 0 0)
    (Transformation|SetActorScale3D "0, 0, 0")
    (Utilities|FlowControl|Sequence
      (:then_0
        ;[1 1 1] Set Scale
        (Components|Activation|SetActive (Variables|Default|GetShield_electro-loop_ver1_1) false true)
        (bind _raidus (Timeline|EquipShield SetNewTime)
          (:Update
            (if (>= (Variables|Default|GetEnergyPoint) 0.0)
              (Transformation|SetActorScale3D (Math|Vector|Lerp(Vector) "0, 0, 0" (stale Custom|SetScale OriginalSize) _raidus))))))
      (:then_1
        ;[1 1 1] Charge
        (Utilities|FlowControl|Gate false) ; enters at Close
      )
      (:then_2
        ;[1 1 1] Be broken
        (Utilities|FlowControl|Delay 5.0)
        (Variables|Default|SetEnergyPoint (* (Variables|Default|GetMaxEnergy) 0.2))
        (Utilities|FlowControl|Gate false) ; enters at Open
      ))))

(event EventBeginPlay
  ;[1 1 1] initialize
  (Variables|Default|SetEnergyPoint (Variables|Default|GetMaxEnergy))
  (bind _returnvalue (Rendering|Material|CreateDynamicMaterialInstance (Variables|Default|GetField) 0 "/Game/Blueprints/ForceField/ForceField_mat_Inst.ForceField_mat_Inst" :!class /Script/Engine.PrimitiveComponent))
  (CallFunction|Charge)
  (CallFunction|Cost))

(fn ConstructionScript)