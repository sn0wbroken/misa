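; ExplodeSpawn is a projectile-driven spawner that turns into an ExplodeEnemy once it drops low enough.
; Shortly after BeginPlay it activates ProjectileMovement and starts a looping timer that checks its altitude.
; Each check rerolls a random height threshold, so the stopping altitude varies between instances.
; At or below the threshold it halts movement, waits briefly, spawns the enemy at its location with random rotation, and destroys itself.
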(event Custom|Altitude%20Test
  (if (<= (.z (Transformation|GetActorLocation)) (Math|Random|RandomFloatinRange 8e+03 5e+04))
    (Components|Activation|SetActive (Variables|Default|GetProjectileMovement) false false)
    (Utilities|FlowControl|Delay 4.0)
    (Game|SpawnActorfromClass "/Game/Blueprints/ExplodeEnemy.ExplodeEnemy_C" (Math|Transform|MakeTransform (Transformation|GetActorLocation) (Math|Random|RandomRotator true) "1,1,1") "Undefined" 0 0)
    (Actor|DestroyActor)))

(event EventBeginPlay
  (Utilities|FlowControl|Delay 0.2)
  (Components|Activation|Activate (Variables|Default|GetProjectileMovement) false)
  (Utilities|Time|SetTimerbyEvent (delegate Custom|Altitude%20Test) 0.5 true))

(fn ConstructionScript)