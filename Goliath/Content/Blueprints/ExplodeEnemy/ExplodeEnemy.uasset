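; Kamikaze enemy that homes in on the player's MISA_Goliath and explodes on contact.
; On BeginPlay it picks a random socket on the player's arm mesh, then each Tick moves forward a fixed, frame-rate-dependent step while interpolating toward it, turning faster when near.
; Trigger overlap with the Goliath damages it, spawns an explosion and applies HP-sized damage to itself.
; The construction script attaches jet particle components to two mesh sockets.
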(event OnComponentBeginOverlap(Triigger)
  (params (OverlappedComponent :type Primitive%20Component%20Object%20Reference) (OtherActor :type Actor%20Object%20Reference) (OtherComp :type Primitive%20Component%20Object%20Reference) (OtherBodyIndex :type Integer) (bFromSweep :type Boolean) (SweepResult :type Hit%20Result%20Structure%20%28by%20ref%29))
  (bind _returnvalue (Transformation|GetActorTransform))
  ;[1 1 1] Self-destroying
  (Utilities|Casting|CastToMISA_Goliath OtherActor)
  (Game|Damage|ApplyDamage OtherActor (Variables|Default|GetDamage) 0 0)
  (Effects|SpawnEmitteratLocation "/Game/StarterContent/Particles/P_Explosion.P_Explosion" (.location _returnvalue) (.rotation _returnvalue) (.scale _returnvalue))
  (Game|Damage|ApplyDamage self (Variables|Default|GetHP) 0 0))

(event EventTick
  (params (DeltaSeconds :type Float%20%28single-precision%29))
  (bind _playerref (Variables|Default|GetPlayerRef))
  ;[1 1 1] Trace
  (if (Variables|Default|GetbActive)
    (Transformation|SetActorLocationAndRotation (+ (Transformation|GetActorLocation) (* (Transformation|GetActorForwardVector) 2e+02)) (Math|Interpolation|RInterpTo (Transformation|GetActorRotation) (Math|Rotator|FindLookatRotation (Transformation|GetActorLocation) (Transformation|GetSocketLocation (Variables|/Game/Blueprints/MISA_Goliath/MISA_Goliath.MISA_Goliath_C|GetArmMesh _playerref) (Variables|Default|GetTarget))) (Utilities|Time|GetWorldDeltaSeconds) (Math|Float|SelectFloat 1.6 0.4 (<= (Transformation|GetDistanceTo _playerref) 5e+04))))
    (else
      (Development|PrintString "stop"))))

(event EventBeginPlay
  ;[1 1 1] initialize
  (bind _asmisa_goliath (Utilities|Casting|CastToMISA_Goliath (Game|Player|GetPlayerPawn 0)))
  (Variables|Default|SetPlayerRef _asmisa_goliath)
  (Variables|Default|SetTarget (Utilities|Array|Get(acopy) (Variables|Default|GetSocket_ary) (Math|Random|RandomIntegerinRange 0 4)))
  (Variables|Default|SetbActive true))

(fn ConstructionScript
  (bind _returnvalue (Math|Transform|MakeTransform "0, 0, 0"))
  (bind _mesh (Variables|Character|GetMesh))
  (bind _returnvalue_2 (AddComponent|AddParticleSystemComponent true _returnvalue))
  (Transformation|AttachComponentToComponent _returnvalue_2 _mesh "Jet" "KeepRelative" "KeepRelative" "KeepRelative" true)
  (bind _returnvalue_3 (AddComponent|AddParticleSystemComponent true _returnvalue))
  (Transformation|AttachComponentToComponent _returnvalue_3 _mesh "JetLower" "KeepRelative" "KeepRelative" "KeepRelative" true))