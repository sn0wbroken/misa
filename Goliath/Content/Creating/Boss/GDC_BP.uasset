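; GDC_BP is a boss Character that makes a dropping entrance with robot voice cues and a heavy landing.
; On BeginPlay it applies a huge downward force through CharacterMovement and plays a distant monster-robot voice, then a second vocal after a delay.
; On landing it activates three particle systems, plays a loud drum impact and a one-shot mesh animation, and sets the IsLand flag.
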(event EventBeginPlay
  (Physics|AddForce (Variables|Character|GetCharacterMovement) "0, 0,-1000000000.000000")
  (Audio|PlaySound2D "/Game/Import/Audio/Robot/MonsterRobot_Voice_Distant01_Cue.MonsterRobot_Voice_Distant01_Cue")
  (Utilities|FlowControl|Delay 4.0)
  (Audio|PlaySound2D "/Game/Import/Audio/Robot/Robot_Vocal03.Robot_Vocal03"))

(event EventOnLanded
  (params (Hit :type Hit%20Result%20Structure%20%28by%20ref%29))
  (Components|Activation|Activate (Variables|Default|GetParticleSystem) false)
  (Audio|PlaySound2D "/Game/Import/Audio/Impact_Drum_Hit_03.Impact_Drum_Hit_03" 5.0)
  (Audio|Components|Audio|Play (Variables|Character|GetMesh) false)
  (Variables|Default|SetbIsLand true))

(fn ConstructionScript)