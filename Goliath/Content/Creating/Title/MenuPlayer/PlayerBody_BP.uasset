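; VR player body for the title menu that handles headset calibration, grip input and revealing a widget on touch.
; Holding ResetVR through a timeline and gate advances a state value, then fades the camera out and recalibrates; early release cancels.
; Calibration, also run at BeginPlay, resets eye-level tracking and scales the body by camera height relative to a Stature reference.
; Keyboard keys mirror the VR inputs and offer a tracking-only reset.
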(event EventBeginPlay
  ;[1 1 1] initialization
  ;[1 1 1] Reset Orientation and Position
  (Class|HeadMountedDisplayFunctionLibrary|SetTrackingOrigin "Eye")
  (Class|HeadMountedDisplayFunctionLibrary|ResetOrientationandPosition 0.0 "OrientationAndPosition") ; 60
  ;[1 1 1] Set the height
  (Transformation|SetRelativeScale3D (Variables|Default|GetBody) (Math|Conversions|ToVector(Float) (/ (.z (.location (Transformation|GetRelativeTransform (Variables|Default|GetCamera)))) (.z (.location (Transformation|GetRelativeTransform (Variables|Default|GetStature))))))))

(event Input|ActionEvents|InputActionAnyTouch
  (params (Key :type Key%20Structure))
  ;[1 1 1] initialization
  (:Pressed
    (Rendering|SetVisibility (Variables|Default|GetWidget) true false)))

(event Input|ActionEvents|InputActionResetVR
  (params (Key :type Key%20Structure))
  ;[1 1 1] Reset Orientation and Position
  (:Pressed
    (Utilities|FlowControl|Sequence
      (:then_0
        (goto _label Open))
      (:then_1
        (bind _direction (Timeline|Hold PlayFromStart)
          (:Update
            (if (Utilities|Enum|Equal(Enum) _direction "Forward")
              (Variables|Default|SetState 1)))
          (:Finished
            (Utilities|FlowControl|Gate true :!label _label
              (:Exit
                (Variables|Default|SetState 2)
                (Utilities|FlowControl|Sequence
                  (:then_0
                    ;[1 1 1] Load
                    (CameraFades|StartCameraFade :self (Game|GetPlayerCameraManager 0) :ToAlpha 1.0 :Duration 3.0 :bHoldWhenFinished true))
                  (:then_1
                    (Class|HeadMountedDisplayFunctionLibrary|SetTrackingOrigin "Eye")
                    (Class|HeadMountedDisplayFunctionLibrary|ResetOrientationandPosition 0.0 "OrientationAndPosition") ; 60
                    ;[1 1 1] Set the height
                    (Transformation|SetRelativeScale3D (Variables|Default|GetBody) (Math|Conversions|ToVector(Float) (/ (.z (.location (Transformation|GetRelativeTransform (Variables|Default|GetCamera)))) (.z (.location (Transformation|GetRelativeTransform (Variables|Default|GetStature))))))))))))))))
  (:Released
    (Utilities|FlowControl|Sequence
      (:then_0
        (goto _label Close))
      (:then_1
        (Timeline|Hold Stop))
      (:then_2
        (if (!= (Variables|Default|GetState) 2)
          (Variables|Default|SetState 0))))))

(event Input|AxisEvents|InputAxisGripLeft
  (params (AxisValue :type Float%20%28single-precision%29))
  ;[1 1 1] Grips
  (Variables|Default|SetARM_Grip_L AxisValue))

(event Input|AxisEvents|InputAxisGripRight
  (params (AxisValue :type Float%20%28single-precision%29))
  ;[1 1 1] Grips
  (Variables|Default|SetARM_Grip_R AxisValue))

(event Input|KeyboardEvents|D
  (params (Key :type Key%20Structure))
  ;[1 1 1] Reset Orientation and Position
  (:Pressed
    (Utilities|FlowControl|Sequence
      (:then_0
        (goto _label Open))
      (:then_1
        (bind _direction (Timeline|Hold PlayFromStart)
          (:Update
            (if (Utilities|Enum|Equal(Enum) _direction "Forward")
              (Variables|Default|SetState 1)))
          (:Finished
            (Utilities|FlowControl|Gate true :!label _label
              (:Exit
                (Variables|Default|SetState 2)
                (Utilities|FlowControl|Sequence
                  (:then_0
                    ;[1 1 1] Load
                    (CameraFades|StartCameraFade :self (Game|GetPlayerCameraManager 0) :ToAlpha 1.0 :Duration 3.0 :bHoldWhenFinished true))
                  (:then_1
                    (Class|HeadMountedDisplayFunctionLibrary|SetTrackingOrigin "Eye")
                    (Class|HeadMountedDisplayFunctionLibrary|ResetOrientationandPosition 0.0 "OrientationAndPosition") ; 60
                    ;[1 1 1] Set the height
                    (Transformation|SetRelativeScale3D (Variables|Default|GetBody) (Math|Conversions|ToVector(Float) (/ (.z (.location (Transformation|GetRelativeTransform (Variables|Default|GetCamera)))) (.z (.location (Transformation|GetRelativeTransform (Variables|Default|GetStature))))))))))))))))
  (:Released
    (Utilities|FlowControl|Sequence
      (:then_0
        (goto _label Close))
      (:then_1
        (Timeline|Hold Stop))
      (:then_2
        (if (!= (Variables|Default|GetState) 2)
          (Variables|Default|SetState 0))))))

(event Input|KeyboardEvents|D
  (params (Key :type Key%20Structure))
  ;[1 1 1] initialization
  (:Pressed
    (Rendering|SetVisibility (Variables|Default|GetWidget) true false)))

(event Input|KeyboardEvents|SpaceBar
  (params (Key :type Key%20Structure))
  ;[1 1 1] Assistant Resest
  (:Pressed
    (Class|HeadMountedDisplayFunctionLibrary|SetTrackingOrigin "Eye")
    (Class|HeadMountedDisplayFunctionLibrary|ResetOrientationandPosition 0.0 "OrientationAndPosition") ; 60
  ))

(fn ConstructionScript)